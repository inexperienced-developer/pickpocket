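; Behavior tree task that picks a random destination for an AI and stores it in the blackboard.
; On execute it gets a random navigable location within Radius of the owner controller's actor location, writes it to BlackboardKey, and finishes with the query's success result.
; A disconnected branch that caches PatrolPoint actors in NavData, plus an unused random pick from that array, remains in the graph but never runs.
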(event `self.ReceiveExecuteAI`
  (params (OwnerController :type "AIController Object Reference") (ControlledPawn :type "Pawn Object Reference"))
  (bind (_randomlocation _returnvalue) (`NavigationSystemV1.K2_GetRandomLocationInNavigableRadius` (`Actor.K2_GetActorLocation` OwnerController) (`self.Radius`) null null))
  (`BTFunctionLibrary.SetBlackboardValueAsVector` (`self.BlackboardKey`) _randomlocation)
  (`self.FinishExecute` _returnvalue))